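; Population manager for a genetic algorithm that evolves Cannon_BP actors over repeated generations, registering itself with CannonMode.
; Spawns the initial population at arrow-component or random in-box transforms, then runs each cannon's sim.
; When all finish, it sorts by fitness, toggles the top cannon's arrow, calls Eliminate and Reproduce, then starts the next generation.
; Repopulate, with its byte-spliced angle crossover and random mutation, is present but never runs.
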(event Custom|RoundFinishedFromPawn
  (bind _population (Variables|Default|GetPopulation))
  (bind _population_2 (Variables|Default|GetPopulation))
  (bind _result (Math|Integer|IncrementInt (Variables|Default|GetNumFinished))
    (:%20%20
      (if (== _result (Variables|Default|GetcurrentSize))
        (CallFunction|FindMostFit _population_2)
        (bind _ascannon_bp (Utilities|Casting|CastToCannon_BP (Utilities|Array|Get(acopy) _population_2)))
        (Rendering|ToggleVisibility (Variables|/Game/ProtoPawns/Cannon/Cannon_BP.Cannon_BP_C|GetThisArrow _ascannon_bp) false)
        (Utilities|FlowControl|Delay 2.0)
        (Class|PopulationActor|Eliminate)
        (Utilities|FlowControl|Delay 3.0)
        (Utilities|Array|Clear (Variables|Default|GetspawnPointArr))
        (if (Variables|Default|GetisLineSpawn?)
          (bind _spawnpoints (CallFunction|RigidSpawn))
          (Class|PopulationActor|Reproduce (Variables|Default|GetPopulation) _spawnpoints)
          (else
            (bind _spawnpoints_2 (CallFunction|RandomSpawn (Variables|Default|GetinitialSize) (Variables|Default|GetcurrentSize)))
            (Variables|Default|SetspawnPointArr _spawnpoints_2)
            (Class|PopulationActor|Reproduce (Variables|Default|GetPopulation) (Variables|Default|GetspawnPointArr))))
        (for _array_element _population
          (bind _ascannon_bp_2 (Utilities|Casting|CastToCannon_BP _array_element))
          (Variables|/Game/ProtoPawns/Cannon/Cannon_BP.Cannon_BP_C|SetcanFire _ascannon_bp_2 true))
        (Variables|Default|SetNumFinished 0)
        (Variables|Default|SetcurrentSize (Utilities|Array|Length _population))
        (CallFunction|EventGA)))))

(event Custom|Event_GA
  (Utilities|FlowControl|Delay 1.0)
  (for _array_element (stale EventBeginPlay _output_get)
    (bind _ascannon_bp (Utilities|Casting|CastToCannon_BP _array_element))
    (Rendering|SetVisibility (Variables|/Game/ProtoPawns/Cannon/Cannon_BP.Cannon_BP_C|GetThisArrow _ascannon_bp) false false))
  (Utilities|FlowControl|Delay 1.0)
  (for _array_element_2 (stale EventBeginPlay _output_get)
    (bind _ascannon_bp_2 (Utilities|Casting|CastToCannon_BP _array_element_2))
    (EventDispatchers|BindEventtoRoundFinished _ascannon_bp_2 (delegate Custom|RoundFinishedFromPawn))
    (Default|RunSim _ascannon_bp_2)))

(event EventBeginPlay
  (Utilities|FlowControl|Delay 1.0)
  (bind _ascannon_mode (Utilities|Casting|CastToCannonMode (Game|GetGameMode)))
  (Variables|/Game/Framework/CannonMode.CannonMode_C|SetPopulationActor _ascannon_mode self)
  (if (Variables|Default|GetisLineSpawn?)
    (bind _spawnpoints (CallFunction|RigidSpawn))
    (Variables|Default|SetspawnPointArr _spawnpoints)
    (else
      (bind _spawnpoints_2 (CallFunction|RandomSpawn (Variables|Default|GetinitialSize)))
      (Variables|Default|SetspawnPointArr _spawnpoints_2)))
  (bind _returnvalue (Class|PopulationActor|PopGenesis (Variables|Default|GetspawnPointArr)))
  (bind _output_get (Variables|Default|SetPopulation _returnvalue))
  (for _array_element _output_get
    (bind _ascannon_bp (Utilities|Casting|CastToCannon_BP _array_element))
    (EventDispatchers|BindEventtoRoundFinished _ascannon_bp (delegate Custom|RoundFinishedFromPawn))
    (Default|RunSim _ascannon_bp)))

(fn ConstructionScript)

(fn RandomBoxTransformPure
  (return (Math|Transform|MakeTransform (Math|Random|RandomPointinBoundingBox (.Location (Math|Transform|BreakTransform (Transformation|GetWorldTransform (Variables|Default|GetDefaultSceneRoot)))) (Variables|/Script/Engine.BoxComponent|GetBoxExtent (Variables|Default|GetBounds))))))

(fn RigidSpawn
  (params (Size :type Integer))
  (for _array_element (Actor|GetComponentsByClass (Utilities|GetClass (Variables|Default|GetArrow)))
    (Utilities|Array|Add (LocalVariables|GetSpawnPts) (Transformation|GetWorldTransform _array_element)))
  (for _array_element_2 (Variables|Default|GetPopulation)
    (bind _ascannon_bp (Utilities|Casting|CastToCannon_BP _array_element_2)
      (:then
        (Utilities|Array|RemoveItem (LocalVariables|GetSpawnPts) (Transformation|GetWorldTransform (Variables|/Game/ProtoPawns/Cannon/Cannon_BP.Cannon_BP_C|GetDefaultSceneRoot _ascannon_bp))))
      (:CastFailed
        (return (LocalVariables|GetSpawnPts)))))
  (return (LocalVariables|GetSpawnPts)))

(fn Comparator
  (params (ObjectA :type Object%20Object%20Reference) (ObjectB :type Object%20Object%20Reference))
  (bind _output_get (LocalVariables|SetLocalObjectA ObjectA))
  (bind _output_get_2 (LocalVariables|SetLocalObjectB ObjectB))
  (bind _asproto_pawn (Utilities|Casting|CastToProtoPawn _output_get))
  (bind _asproto_pawn_2 (Utilities|Casting|CastToProtoPawn _output_get_2))
  (return (< (Variables|/Script/Protolith.ProtoPawn|Getfitness _asproto_pawn) (Variables|/Script/Protolith.ProtoPawn|Getfitness _asproto_pawn_2))))

(fn FindMostFit
  (params (ProtoPawns :type Array%20of%20Object%20Object%20References))
  (Class|LowEntryExtendedStandardLibrary|SortObjectArrayDirectly ProtoPawns (EventDispatchers|CreateEvent :!event Comparator) true)
  (return))

(fn RandomSpawn
  (params (NumToSpawn :type Integer) (First :type Integer))
  (for _index (range 0 (- NumToSpawn 1))
    (Utilities|Array|Add (Variables|Default|GetspawnPointArr) (CallFunction|RandomBoxTransformPure)))
  (return (Variables|Default|GetspawnPointArr)))

(fn Repopulate
  (params (SpawnPts :type Array%20of%20Transforms))
  (for _array_element SpawnPts
    (bind _returnvalue (Game|SpawnActorfromClass "/Game/ProtoPawns/Cannon/Cannon_BP.Cannon_BP_C" _array_element "AdjustIfPossibleButAlwaysSpawn" 0 0))
    (Utilities|Array|Add (Variables|Default|GetPopulation) _returnvalue)
    (bind _output_get (CallFunction|MutateAngle))
    (bind _output_get_2 (Variables|/Game/ProtoPawns/Cannon/Cannon_BP.Cannon_BP_C|SetCannonAngle _returnvalue _output_get))
    (Default|SetCannonAngle _returnvalue _output_get_2))
  (return))

(fn MutateAngle
  (bind _ascannon_bp (Utilities|Casting|CastToCannon_BP (Utilities|Array|Get(acopy) (Variables|Default|GetPopulation) (Math|Random|RandomIntegerinRange 0 (Variables|Default|GetcurrentSize)))))
  (bind _output_get (LocalVariables|Setparent1 (Class|LowEntryExtendedStandardLibrary|FloattoBytes (Variables|/Game/ProtoPawns/Cannon/Cannon_BP.Cannon_BP_C|GetCannonAngle _ascannon_bp))))
  (bind _ascannon_bp_2 (Utilities|Casting|CastToCannon_BP (Utilities|Array|Get(acopy) (Variables|Default|GetPopulation) (Math|Random|RandomIntegerinRange 0 (Variables|Default|GetcurrentSize)))))
  (bind _output_get_2 (LocalVariables|Setparent2 (Class|LowEntryExtendedStandardLibrary|FloattoBytes (Variables|/Game/ProtoPawns/Cannon/Cannon_BP.Cannon_BP_C|GetCannonAngle _ascannon_bp_2))))
  (return (+ (Class|LowEntryExtendedStandardLibrary|BytestoFloat (|LowEntryMergeBytesPure (.A (Class|LowEntryExtendedStandardLibrary|SplitBytes _output_get 2)) (.A (Class|LowEntryExtendedStandardLibrary|SplitBytes _output_get_2 2)) (.B (Class|LowEntryExtendedStandardLibrary|SplitBytes _output_get 2)) (.B (Class|LowEntryExtendedStandardLibrary|SplitBytes _output_get_2 2)))) (Math|Random|RandomFloatinRange -5.0 5.0))))