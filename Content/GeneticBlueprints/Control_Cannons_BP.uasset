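; Control-group manager for a genetic cannon experiment, spawning one random and one deterministic control cannon.
; Each round it increments non-random cannons' DetermAngle, runs both sims, waits for their finished events, then re-arms them after delays and loops.
; CannonMode's ParamControl StartStop event pauses the loop, and a Location stage index selects where it resumes.
; Fitness-sort, repopulation and byte-crossover mutation functions exist but are unused by this loop.
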(event Custom|RoundFinishedFromPawn
  (bind _result (Math|Integer|IncrementInt (Variables|Default|GetNumFinished))
    (:%20%20
      (if (== _result (Variables|Default|GetcurrentSize))
        (if (Variables|Default|GetisRunning)
          (Variables|Default|SetLocation 2)
          (Utilities|FlowControl|Delay 2.0)
          (if (Variables|Default|GetisRunning)
            (Variables|Default|SetLocation 3)
            (Utilities|FlowControl|Delay 3.0)
            (if (Variables|Default|GetisRunning)
              (Variables|Default|SetLocation 4)
              (Variables|Default|SetNumFinished 0)
              (for _array_element (Variables|Default|GetControlPop)
                (Variables|/Game/ProtoPawns/Cannon/ControlCannon_BP.ControlCannon_BP_C|SetcanFire _array_element true))
              (CallFunction|EventGA))))))))

(event Custom|Event_GA
  (Utilities|FlowControl|Delay 1.0)
  (if (Variables|Default|GetisRunning)
    (Variables|Default|SetLocation 1)
    (for _array_element (Variables|Default|GetControlPop)
      (bind _ascontrol_cannon_bp (Utilities|Casting|CastToControlCannon_BP _array_element))
      (if (Variables|/Game/ProtoPawns/Cannon/ControlCannon_BP.ControlCannon_BP_C|GetisRandom _ascontrol_cannon_bp)
        _
        (else
          (Math|Integer|IncrementInt (Variables|/Game/ProtoPawns/Cannon/ControlCannon_BP.ControlCannon_BP_C|GetDetermAngle _ascontrol_cannon_bp)
            (:%20%20
              _))))
      (EventDispatchers|BindEventtoRoundFinished _ascontrol_cannon_bp (delegate Custom|RoundFinishedFromPawn))
      (Default|RunSim _ascontrol_cannon_bp))))

(event Custom|Start0
  (if (Variables|Default|GetisRunning)
    (Variables|Default|SetLocation 1)
    (CallFunction|RigidSpawn)
    (for _array_element (Variables|Default|GetControlPop)
      (bind _ascontrol_cannon_bp (Utilities|Casting|CastToControlCannon_BP _array_element))
      (if (Variables|/Game/ProtoPawns/Cannon/ControlCannon_BP.ControlCannon_BP_C|GetisRandom _ascontrol_cannon_bp)
        _
        (else
          (Math|Integer|IncrementInt (Variables|/Game/ProtoPawns/Cannon/ControlCannon_BP.ControlCannon_BP_C|GetDetermAngle _ascontrol_cannon_bp)
            (:%20%20
              _))))
      (EventDispatchers|BindEventtoRoundFinished _ascontrol_cannon_bp (delegate Custom|RoundFinishedFromPawn))
      (Default|RunSim _ascontrol_cannon_bp))))

(event Custom|Start1
  (if (Variables|Default|GetisRunning)
    (Variables|Default|SetLocation 2)
    (Utilities|FlowControl|Delay 2.0)
    (if (Variables|Default|GetisRunning)
      (Variables|Default|SetLocation 3)
      (Utilities|FlowControl|Delay 3.0)
      (if (Variables|Default|GetisRunning)
        (Variables|Default|SetLocation 4)
        (Variables|Default|SetNumFinished 0)
        (for _array_element (Variables|Default|GetControlPop)
          (Variables|/Game/ProtoPawns/Cannon/ControlCannon_BP.ControlCannon_BP_C|SetcanFire _array_element true))
        (CallFunction|EventGA)))))

(event Custom|Start2
  (if (Variables|Default|GetisRunning)
    (Variables|Default|SetLocation 3)
    (Utilities|FlowControl|Delay 3.0)
    (if (Variables|Default|GetisRunning)
      (Variables|Default|SetLocation 4)
      (Variables|Default|SetNumFinished 0)
      (for _array_element (Variables|Default|GetControlPop)
        (Variables|/Game/ProtoPawns/Cannon/ControlCannon_BP.ControlCannon_BP_C|SetcanFire _array_element true))
      (CallFunction|EventGA))))

(event Custom|StartStop
  (params (Start :type Boolean))
  (bind _output_get (Variables|Default|SetIsRunning Start))
  (if _output_get
    (switch int (Variables|Default|GetLocation)
      (:Default
        (CallFunction|Start0 :!label _label))
      (:0
        (goto _label))
      (:1
        (CallFunction|Start1))
      (:2
        (CallFunction|Start2))
      (:3
        (CallFunction|Start3))
      (:4
        (CallFunction|Start4)))))

(event Custom|Start3
  (if (Variables|Default|GetisRunning)
    (Variables|Default|SetLocation 4)
    (Variables|Default|SetNumFinished 0)
    (for _array_element (Variables|Default|GetControlPop)
      (Variables|/Game/ProtoPawns/Cannon/ControlCannon_BP.ControlCannon_BP_C|SetcanFire _array_element true))
    (CallFunction|EventGA)))

(event Custom|Start4
  (if (Variables|Default|GetisRunning)
    (Variables|Default|SetLocation 1)
    (for _array_element (Variables|Default|GetControlPop)
      (bind _ascontrol_cannon_bp (Utilities|Casting|CastToControlCannon_BP _array_element))
      (if (Variables|/Game/ProtoPawns/Cannon/ControlCannon_BP.ControlCannon_BP_C|GetisRandom _ascontrol_cannon_bp)
        _
        (else
          (Math|Integer|IncrementInt (Variables|/Game/ProtoPawns/Cannon/ControlCannon_BP.ControlCannon_BP_C|GetDetermAngle _ascontrol_cannon_bp)
            (:%20%20
              _))))
      (EventDispatchers|BindEventtoRoundFinished _ascontrol_cannon_bp (delegate Custom|RoundFinishedFromPawn))
      (Default|RunSim _ascontrol_cannon_bp))))

(event EventBeginPlay
  (Variables|Default|SetisRunning true)
  (Variables|Default|SetLocation 0)
  (Utilities|FlowControl|Delay 0.06)
  (bind _ascannon_mode (Utilities|Casting|CastToCannonMode (Game|GetGameMode)))
  (EventDispatchers|BindEventtoStartStop (Variables|/Game/Framework/CannonMode.CannonMode_C|GetParamControl _ascannon_mode) (delegate Custom|StartStop))
  (if (Variables|Default|GetisRunning)
    (Variables|Default|SetLocation 1)
    (CallFunction|RigidSpawn)
    (for _array_element (Variables|Default|GetControlPop)
      (bind _ascontrol_cannon_bp (Utilities|Casting|CastToControlCannon_BP _array_element))
      (if (Variables|/Game/ProtoPawns/Cannon/ControlCannon_BP.ControlCannon_BP_C|GetisRandom _ascontrol_cannon_bp)
        _
        (else
          (Math|Integer|IncrementInt (Variables|/Game/ProtoPawns/Cannon/ControlCannon_BP.ControlCannon_BP_C|GetDetermAngle _ascontrol_cannon_bp)
            (:%20%20
              _))))
      (EventDispatchers|BindEventtoRoundFinished _ascontrol_cannon_bp (delegate Custom|RoundFinishedFromPawn))
      (Default|RunSim _ascontrol_cannon_bp))))

(fn ConstructionScript)

(fn RandomBoxTransformPure
  (return (Math|Transform|MakeTransform (Math|Random|RandomPointinBoundingBox (.Location (Math|Transform|BreakTransform (Transformation|GetWorldTransform (Variables|Default|GetDefaultSceneRoot)))) (Variables|/Script/Engine.BoxComponent|GetBoxExtent (Variables|Default|GetBounds))))))

(fn RigidSpawn
  (bind _returnvalue (Game|SpawnActorfromClass "/Game/ProtoPawns/Cannon/ControlCannon_BP.ControlCannon_BP_C" (Transformation|GetWorldTransform (Variables|Default|GetRandom)) "Undefined" 0 0))
  (bind _output_get (Variables|Default|SetRandomCannon _returnvalue))
  (Rendering|Material|SetMaterial (Variables|/Game/ProtoPawns/Cannon/ControlCannon_BP.ControlCannon_BP_C|GetCannonMesh _output_get) 2 "/Game/ProtoPawns/Cannon/Materials/ControlCannon_Random_Inst.ControlCannon_Random_Inst")
  (Utilities|Array|Add (Variables|Default|GetControlPop) _output_get)
  (bind _returnvalue_2 (Game|SpawnActorfromClass "/Game/ProtoPawns/Cannon/ControlCannon_BP.ControlCannon_BP_C" (Transformation|GetWorldTransform (Variables|Default|GetDeterministic)) "Undefined" 0 0))
  (Rendering|Material|SetMaterial (Variables|/Game/ProtoPawns/Cannon/ControlCannon_BP.ControlCannon_BP_C|GetCannonMesh _returnvalue_2) 2 "/Game/ProtoPawns/Cannon/Materials/ControlCannon_Inst.ControlCannon_Inst")
  (Variables|/Script/Engine.Actor|SetTags _returnvalue_2 (Variables|Default|GetRandomTag))
  (bind _output_get_2 (Variables|Default|SetDetermCannon _returnvalue_2))
  (Utilities|Array|Add (Variables|Default|GetControlPop) _output_get_2)
  (Variables|Default|SetcurrentSize (Utilities|Array|Length (Variables|Default|GetControlPop))))

(fn Comparator
  (params (ObjectA :type Object%20Object%20Reference) (ObjectB :type Object%20Object%20Reference))
  (bind _output_get (LocalVariables|SetLocalObjectA ObjectA))
  (bind _output_get_2 (LocalVariables|SetLocalObjectB ObjectB))
  (bind _asproto_pawn (Utilities|Casting|CastToProtoPawn _output_get))
  (bind _asproto_pawn_2 (Utilities|Casting|CastToProtoPawn _output_get_2))
  (return (< (Variables|/Script/Protolith.ProtoPawn|Getfitness _asproto_pawn) (Variables|/Script/Protolith.ProtoPawn|Getfitness _asproto_pawn_2))))

(fn FindMostFit
  (params (ProtoPawns :type Array%20of%20Object%20Object%20References))
  (Class|LowEntryExtendedStandardLibrary|SortObjectArrayDirectly ProtoPawns (EventDispatchers|CreateEvent :!event Comparator) true)
  (return))

(fn RandomSpawn
  (params (NumToSpawn :type Integer))
  (for _index (range 1 NumToSpawn)
    (Utilities|Array|Add (Variables|Default|GetspawnPointArr) (CallFunction|RandomBoxTransformPure)))
  (return (Variables|Default|GetspawnPointArr)))

(fn Repopulate
  (params (SpawnPts :type Array%20of%20Transforms))
  (for _array_element SpawnPts
    (bind _returnvalue (Game|SpawnActorfromClass "/Game/ProtoPawns/Cannon/Cannon_BP.Cannon_BP_C" _array_element "AdjustIfPossibleButAlwaysSpawn" 0 0))
    (Utilities|Array|Add (Variables|Default|GetPopulation) _returnvalue)
    (bind _output_get (CallFunction|MutateAngle))
    (bind _output_get_2 (Variables|/Game/ProtoPawns/Cannon/Cannon_BP.Cannon_BP_C|SetCannonAngle _returnvalue _output_get))
    (Default|SetCannonAngle _returnvalue _output_get_2))
  (return))

(fn MutateAngle
  (bind _ascannon_bp (Utilities|Casting|CastToCannon_BP (Utilities|Array|Get(acopy) (Variables|Default|GetPopulation) (Math|Random|RandomIntegerinRange 0 (Variables|Default|GetcurrentSize)))))
  (bind _output_get (LocalVariables|Setparent1 (Class|LowEntryExtendedStandardLibrary|FloattoBytes (Variables|/Game/ProtoPawns/Cannon/Cannon_BP.Cannon_BP_C|GetCannonAngle _ascannon_bp))))
  (bind _ascannon_bp_2 (Utilities|Casting|CastToCannon_BP (Utilities|Array|Get(acopy) (Variables|Default|GetPopulation) (Math|Random|RandomIntegerinRange 0 (Variables|Default|GetcurrentSize)))))
  (bind _output_get_2 (LocalVariables|Setparent2 (Class|LowEntryExtendedStandardLibrary|FloattoBytes (Variables|/Game/ProtoPawns/Cannon/Cannon_BP.Cannon_BP_C|GetCannonAngle _ascannon_bp_2))))
  (return (+ (Class|LowEntryExtendedStandardLibrary|BytestoFloat (|LowEntryMergeBytesPure (.A (Class|LowEntryExtendedStandardLibrary|SplitBytes _output_get 2)) (.A (Class|LowEntryExtendedStandardLibrary|SplitBytes _output_get_2 2)) (.B (Class|LowEntryExtendedStandardLibrary|SplitBytes _output_get 2)) (.B (Class|LowEntryExtendedStandardLibrary|SplitBytes _output_get_2 2)))) (Math|Random|RandomFloatinRange -5.0 5.0))))