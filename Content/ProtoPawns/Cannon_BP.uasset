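; Prototype cannon Blueprint with a poseable barrel and unfinished firing logic.
; The construction script rotates the barrel bone to CannonAngle in world space.
; BeginPlay and FireCannon are empty.
; Disconnected nodes sketch aiming the barrel, spawning a CannonBall at the barrel socket and applying a Force-scaled impulse, though the impulse vector is zero, and none of it runs.
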(event EventBeginPlay)

(fn ConstructionScript
  (Components|PoseableMesh|SetBoneRotationbyName (Variables|Default|GetCannonMesh) (Variables|Default|GetBarrelBoneName) (Math|Rotator|MakeRotator (Variables|Default|GetCannonAngle) 0.0 0.0) "WorldSpace"))

(fn FireCannon)