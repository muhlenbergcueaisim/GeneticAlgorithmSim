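; Simulation cannon that fires a series of cannonballs at one barrel angle and scores it by average shot distance.
; RunSim picks a random angle for "RandomCannon"-tagged actors or an incrementing one otherwise, poses the barrel bone, then fires each second until MaxShots.
; Shots are pushed along the bone-to-bone vector and report landing distances; the last landing sets Fitness and calls RoundFinished.
; Player-facing FitnessText displays the angle, despite its name.
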(event Custom|RunSim
  (if (Actor|ActorHasTag self "RandomCannon")
    (CallFunction|SetCannonAngle (Math|Conversions|ToFloat(Integer) (Math|Random|RandomIntegerinRange 0 90)))
    (else
      (CallFunction|SetCannonAngle (Math|Conversions|ToFloat(Integer) (Variables|Default|GetDetermAngle)))
      (Math|Integer|IncrementInt (Variables|Default|GetDetermAngle)
        (:%20%20
          _))))
  (if (Variables|Default|GetcanFire) :!label _label
    (CallFunction|FireCannon)
    (EventDispatchers|BindEventtoShotLanded (Variables|Default|GetCannonBall) (delegate Custom|CannonShotLanded))
    (Utilities|FlowControl|RetriggerableDelay 1.0)
    (goto _label)))

(event Custom|CannonShotLanded
  (params (DistanceIn :type Float%20%28single-precision%29))
  (CallFunction|ShotLandedEvent DistanceIn))

(event EventTick
  (params (DeltaSeconds :type Float%20%28single-precision%29))
  (bind _fitnesstext (Variables|Default|GetFitnessText))
  (Transformation|SetWorldRotation _fitnesstext (Transformation|GetActorRotation (Game|GetPlayerController 0)) false false)
  (Transformation|AddLocalRotation _fitnesstext "0,180.000000, 0" false false))

(fn ConstructionScript)

(fn FireCannon
  (bind _self self)
  (bind _returnvalue (Class|PoseableMeshComponent|GetBoneTransformbyName (Variables|Default|GetCannonMesh) (Variables|Default|GetBarrelBoneNameEnd) "WorldSpace"))
  (LocalVariables|SetBarrelTransform "")
  (bind _returnvalue_2 (Game|SpawnActorfromClass "/Game/ProtoPawns/Cannon/CannonBall.CannonBall_C" (Math|Transform|MakeTransform (.location _returnvalue) "0, 0, 0" "1,1,1") "AlwaysSpawn" _self _self))
  (Variables|Default|SetCannonBall _returnvalue_2)
  (Effects|SpawnEmitteratLocation "/Game/Particles/P_Explosion.P_Explosion" (.location _returnvalue))
  (Variables|/Game/ProtoPawns/Cannon/CannonBall.CannonBall_C|SetOwningCannon _returnvalue_2 self)
  (Physics|AddForce (Variables|/Game/ProtoPawns/Cannon/CannonBall.CannonBall_C|GetCannonShot (Variables|Default|GetCannonBall)) (* (Variables|Default|GetFireForward) (Variables|Default|GetForce)) "None" false)
  (bind _result (Math|Integer|IncrementInt (Variables|Default|GetnumShots))
    (:%20%20
      (if (== _result (Variables|Default|GetmaxShots))
        (Variables|Default|SetcanFire false)
        (Variables|Default|SetnumShots 0)
        (return)))))

(fn EvaluateFitness
  (params (TotalDistance :type Float%20%28single-precision%29) (numShot :type Integer))
  (return (/ TotalDistance (Math|Conversions|ToFloat(Integer) numShot))))

(fn ShotLandedEvent
  (params (Distance :type Float%20%28single-precision%29))
  (Variables|Default|SetTotalDistance (+ Distance (Variables|Default|GetTotalDistance)))
  (bind _result (Math|Integer|IncrementInt (Variables|Default|GetshotsLanded))
    (:%20%20
      (if (== _result (Variables|Default|GetmaxShots))
        (bind _fitnessout (CallFunction|EvaluateFitness (Variables|Default|GetTotalDistance) (Variables|Default|GetshotsLanded)))
        (Variables|Default|Setfitness _fitnessout)
        (bind _output_get (Variables|Default|SetisFinished true))
        (if _output_get
          (Variables|Default|SetshotsLanded 0)
          (Variables|Default|SetTotalDistance 0.0)
          (Default|CallRoundFinished))))))

(fn SetCannonAngle
  (params (inAngle :type Float%20%28single-precision%29))
  (Variables|Default|SetCannonAngle inAngle)
  (bind _returnvalue (Class|PoseableMeshComponent|GetBoneRotationbyName (Variables|Default|GetCannonMesh) (Variables|Default|GetBarrelBoneName) "WorldSpace"))
  (Components|PoseableMesh|SetBoneRotationbyName (Variables|Default|GetCannonMesh) (Variables|Default|GetBarrelBoneName) (Math|Rotator|MakeRotator (.roll _returnvalue) (Variables|Default|GetCannonAngle) (.yaw _returnvalue)) "WorldSpace")
  (bind _returnvalue_2 (Class|PoseableMeshComponent|GetBoneLocationbyName (Variables|Default|GetCannonMesh) (Variables|Default|GetBarrelBoneName) "WorldSpace"))
  (Variables|Default|SetBoneForward _returnvalue_2)
  (bind _returnvalue_3 (Class|PoseableMeshComponent|GetBoneLocationbyName (Variables|Default|GetCannonMesh) (Variables|Default|GetBarrelBoneNameEnd) "WorldSpace"))
  (bind _output_get (Variables|Default|SetBoneForwardEnd _returnvalue_3))
  (Variables|Default|SetFireForward (- _output_get (Variables|Default|GetBoneForward)))
  (Rendering|Components|TextRender|SetText (Variables|Default|GetFitnessText) (Utilities|Text|ToText(Float) (Variables|Default|GetCannonAngle) "HalfToEven" false true 1 324 0 1)))