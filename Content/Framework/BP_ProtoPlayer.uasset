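; BP_ProtoPlayer is the prototype player Blueprint, handling camera switching, chart display and simulation saves for the CannonMode game mode.
; BeginPlay gathers all level CameraActors and caches CannonMode; Space steps through those cameras with an eased blend.
; Holding C shows the game mode's chart.
; SaveSim writes a freshly created, unpopulated SaveObject_BP to the named slot, and LoadGenerations returns the stored Generations from that slot.
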(event Custom|SaveSim
  (params (FileName :type String))
  (Variables|Default|SetSlotName FileName)
  (bind _returnvalue (SaveGame|CreateSaveGameObject "/Game/Framework/SaveObject_BP.SaveObject_BP_C"))
  (SaveGame|SaveGametoSlot _returnvalue (Variables|Default|GetSlotName)))

(event EventBeginPlay
  (bind _outactors (Actor|GetAllActorsOfClass "/Script/Engine.CameraActor"))
  (Variables|Default|SetCameraRefs _outactors)
  (bind _ascannon_mode (Utilities|Casting|CastToCannonMode (Game|GetGameMode)))
  (Variables|Default|SetCannonMode _ascannon_mode))

(event EventTick
  (params (DeltaSeconds :type Float%20%28single-precision%29)))

(event Input|KeyboardEvents|SpaceBar
  (params (Key :type Key%20Structure))
  (bind _camerarefs (Variables|Default|GetCameraRefs))
  (:Pressed
    (if (>= (Variables|Default|GetCurrentCamNum) (Utilities|Array|Length _camerarefs))
      (Variables|Default|SetCurrentCamNum 0)
      (else
        (bind _result (Math|Integer|IncrementInt (Variables|Default|GetCurrentCamNum))
          (:%20%20
            _))))
    (Game|Player|SetViewTargetwithBlend (Utilities|Array|Get(acopy) _camerarefs _result) 1.0 "VTBlend_EaseIn" 0.0 false)))

(event Input|KeyboardEvents|C
  (params (Key :type Key%20Structure))
  (:Pressed
    (Default|DisplayChart (Variables|Default|GetCannonMode)))
  (:Released
    (Default|HideChart (Variables|Default|GetCannonMode))))

(fn ConstructionScript)

(fn LoadGenerations
  (bind _returnvalue (SaveGame|LoadGamefromSlot (Variables|Default|GetSlotName)))
  (bind _assave_object_bp (Utilities|Casting|CastToSaveObject_BP _returnvalue))
  (return (Variables|/Game/Framework/SaveObject_BP.SaveObject_BP_C|GetGenerations _assave_object_bp)))