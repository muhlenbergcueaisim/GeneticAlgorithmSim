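; PopulationActor is a spawner that creates an initial population of ProtoPawn_BP actors when play begins.
; BeginPlay loops over InitialSize, spawning a pawn at a random transform, clearing the ProtoPawn variable and printing a debug message each pass.
; RandomBoxTransform picks a random point in a box centered on the scene root, sized by the Bounds extent, with zero rotation and unit scale.
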(event EventBeginPlay
  (for _index (range 0 (Variables|Default|GetinitialSize))
    (bind _spawntransform (CallFunction|RandomBoxTransform))
    (Game|SpawnActorfromClass "/Game/ProtoPawn_BP.ProtoPawn_BP_C" _spawntransform "Undefined" 0 0)
    (Variables|Default|SetProtoPawn 0)
    (Development|PrintString "Hello")))

(event EventTick
  (params (DeltaSeconds :type Float%20%28single-precision%29)))

(fn ConstructionScript)

(fn RandomBoxTransform
  (return (Math|Transform|MakeTransform (Math|Random|RandomPointinBoundingBox (.Location (Math|Transform|BreakTransform (Transformation|GetWorldTransform (Variables|Default|GetDefaultSceneRoot)))) (Variables|/Script/Engine.BoxComponent|GetBoxExtent (Variables|Default|GetBounds))))))